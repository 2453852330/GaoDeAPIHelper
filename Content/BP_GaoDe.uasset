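; BP_GaoDe is a demo actor for GaoDe weather and IP lookup queries.
; On BeginPlay it shows the mouse cursor and creates the UI_GaoDe widget, passing itself as a reference.
; BPI query events call QueryWeather, in base or full mode, and QueryIp.
; Finish and error events print the returned weather, IP or error info to screen, with full weather showing only location, report time and forecast count.
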(event `/GaoDeAPIHelper/BPI_GaoDe.BPI_QueryWeather`
  (params (bBase :type Boolean) (CityCode :type String))
  ;[0.9922 0 1] weather
  (if bBase
    (`self.QueryWeather` CityCode "EBase")
    (else
      (`self.QueryWeather` CityCode "EAll"))))

(event `self.BPQueryWeatherFinishBase`
  (params (Weather :type "WeatherBase Structure (by ref)"))
  ;[0.9922 0 1] weather
  (`KismetSystemLibrary.PrintString` (`GaoDeLib.WeatherBaseToString` Weather) true true (struct :`G` 0.66 :`B` 1.0 :`A` 1.0) 20.0))

(event `self.BPReceiveErrorInfo`
  (params (ErrorInfo :type String))
  ;[0.3359 1 0] error
  (`KismetSystemLibrary.PrintString` ErrorInfo))

(event `self.BPQueryWeatherFinishAll`
  (params (Weather :type "WeatherAll Structure (by ref)"))
  (bind (_province _city _adcode _reporttime _casts) (break `WeatherAll` Weather))
  ;[0.9922 0 1] weather
  (`KismetSystemLibrary.PrintText` (`|FormatText` "{a} | {b} | {c} | {d} | {e}" _province _city _adcode _reporttime (`KismetArrayLibrary.Array_Length` _casts))))

(event `self.ReceiveBeginPlay`
  (bind _returnvalue (`GameplayStatics.GetPlayerController` 0))
  ;[0.1719 0 1] begin
  (set `PlayerController.bShowMouseCursor` true _returnvalue)
  (bind _returnvalue_2 (`|CreateWidget` "/GaoDeAPIHelper/UI_GaoDe.UI_GaoDe_C" _returnvalue self))
  (`UserWidget.AddToViewport` _returnvalue_2 0))

(event `/GaoDeAPIHelper/BPI_GaoDe.BPI_QueryIP`
  (params (Ip :type String))
  ;[0 1 0.25] ip
  (`self.QueryIp` Ip))

(event `self.BPQueryIpFinish`
  (params (IpInfo :type "IpType Structure (by ref)"))
  ;[0 1 0.25] ip
  (`KismetSystemLibrary.PrintString` (`GaoDeLib.IpToString` IpInfo)))

(fn `UserConstructionScript`)